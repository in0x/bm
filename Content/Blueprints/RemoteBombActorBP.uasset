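; Remote bomb actor that explodes when its owning player character triggers it.
; On BeginPlay it casts its Instigator to BmPlayerCharacter and binds to that character's remote-bomb-triggered event, printing an error if the cast fails.
; When the event names this bomb, it unbinds from the character and calls ExplodeImplementation, so other bombs listening to the same event stay intact.
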(event Custom|BombTriggered
  (params (TriggeredBomb :type Bm%20Base%20Bomb%20Actor%20Object%20Reference))
  ;[1 1 1] Event BombTriggered
  (if (== TriggeredBomb self)
    (bind _asbm_player_character (Utilities|Casting|CastToBmPlayerCharacter (Variables|Default|GetInstigator)))
    (EventDispatchers|UnbindEventfromRemoteBombTriggered _asbm_player_character (delegate Custom|BombTriggered))
    (Class|BmBaseBombActor|ExplodeImplementation)))

(event EventBeginPlay
  ;[1 1 1] BeginPlay()
  (bind _asbm_player_character (Utilities|Casting|CastToBmPlayerCharacter (Variables|Default|GetInstigator))
    (:then
      (EventDispatchers|BindEventtoRemoteBombTriggered _asbm_player_character (delegate Custom|BombTriggered)))
    (:CastFailed
      (Development|PrintText "Failed to cast TimedBomb Instigator to BmPlayerCharacter"))))

(event Collision|EventActorBeginOverlap
  (params (OtherActor :type Actor%20Object%20Reference)))

(event EventTick
  (params (DeltaSeconds :type Float%20%28single-precision%29)))

(fn ConstructionScript)