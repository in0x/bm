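; Game mode Blueprint that presents the end-of-round result for a multiplayer match and handles restarting.
; On BeginPlay it binds the restart button in the Overlay user widget, held by a widget component, to RestartGame.
; The GameEndedWin and GameEndedDraw events write the winning player's ID or a draw message into the overlay, then reveal the widget and button.
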(event Custom|OnRestartClicked
  (Class|BmGameMode|RestartGame))

(event EventBeginPlay
  (bind _asoverlay (Utilities|Casting|CastToOverlay (UserInterface|GetUserWidgetObject (Variables|Default|GetWidget))))
  (EventDispatchers|BindEventtoOnClicked (Variables|/Game/Blueprints/UI/Overlay.Overlay_C|GetButton_0 _asoverlay) (delegate Custom|OnRestartClicked)))

(event EventGameEndedWin
  (params (WinningPlayerID :type Integer))
  ;[1 1 1] Set Screen Text for Winner
  (bind _asoverlay (Utilities|Casting|CastToOverlay (UserInterface|GetUserWidgetObject (Variables|Default|GetWidget))))
  (Variables|/Game/Blueprints/UI/Overlay.Overlay_C|SetEndOfRoundText _asoverlay (Utilities|String|ToString(Text) (Utilities|Text|FormatText "Player {ID} won!" WinningPlayerID)))
  (Rendering|SetVisibility (Variables|Default|GetWidget) true false)
  (Widget|SetVisibility (Variables|/Game/Blueprints/UI/Overlay.Overlay_C|GetButton_0 _asoverlay) "Visible"))

(event EventGameEndedDraw
  ;[1 1 1] Set Screen Text for Draw
  (bind _asoverlay (Utilities|Casting|CastToOverlay (UserInterface|GetUserWidgetObject (Variables|Default|GetWidget))))
  (Variables|/Game/Blueprints/UI/Overlay.Overlay_C|SetEndOfRoundText _asoverlay "It's a draw!")
  (Rendering|SetVisibility (Variables|Default|GetWidget) true false)
  (Widget|SetVisibility (Variables|/Game/Blueprints/UI/Overlay.Overlay_C|GetButton_0 _asoverlay) "Visible"))

(fn ConstructionScript)