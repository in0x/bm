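; Pickup actor that temporarily switches the collecting character's bombs to remote bombs.
; On pickup it stores the character, sets its bomb class to RemoteBombActorBP, starts a ten-second timer, unbinds its overlap events and hides its mesh.
; The hidden actor stays alive until the timer fires PickupElapsed, which sets the bomb class to TimedBombActorBP rather than restoring the previous one, then destroys the pickup.
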(event EventBeginPlay)

(event Collision|EventActorBeginOverlap
  (params (OtherActor :type Actor%20Object%20Reference)))

(event EventOnCharacterPickedUp
  (params (Character :type Bm%20Player%20Character%20Object%20Reference))
  ;[1 1 1] Set Bomb Class to Remote and start timer
  (bind _output_get (Variables|Default|SetUsingPlayer Character))
  (Class|BmPlayerCharacter|SetBombClass _output_get "/Game/Blueprints/RemoteBombActorBP.RemoteBombActorBP_C")
  (bind _returnvalue (Utilities|Time|SetTimerbyFunctionName 0 "PickupElapsed" 1e+01))
  (Variables|Default|SetTimer _returnvalue)
  ;[1 1 1] Unbind Overlap CB and set invisible
  (EventDispatchers|UnbindallEventsfromOnActorBeginOverlap)
  (Rendering|SetVisibility (Variables|Default|GetStaticMeshComponent) false true))

(event EventTick
  (params (DeltaSeconds :type Float%20%28single-precision%29)))

(fn ConstructionScript)

(fn PickupElapsed
  (Class|BmPlayerCharacter|SetBombClass (Variables|Default|GetUsingPlayer) "/Game/Blueprints/TimedBombActorBP.TimedBombActorBP_C")
  (Utilities|Time|ClearandInvalidateTimerbyHandle (Variables|Default|GetTimer))
  (Actor|DestroyActor))