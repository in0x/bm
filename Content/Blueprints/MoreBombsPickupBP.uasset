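; MoreBombsPickupBP is a pickup that increases how many bombs a character can have.
; When the OnCharacterPickedUp event fires, it adds BombCountIncrease to the character's max bomb count, then destroys itself.
; BeginPlay and the construction script only call their parent versions, and the overlap and tick events are disabled.
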(event EventBeginPlay
  (|CallParentFunction))

(event Collision|EventActorBeginOverlap
  (params (OtherActor :type Actor%20Object%20Reference))
  (|CallParentFunction OtherActor))

(event EventOnCharacterPickedUp
  (params (Character :type Bm%20Player%20Character%20Object%20Reference))
  ;[1 1 1] Event OnCharacterPickedUp
  (bind _returnvalue (Class|BmPlayerCharacter|GetMaxBombCount Character))
  (Class|BmPlayerCharacter|SetMaxBombCount Character (+ _returnvalue (Variables|Default|GetBombCountIncrease)))
  (Actor|DestroyActor))

(event EventTick
  (params (DeltaSeconds :type Float%20%28single-precision%29))
  (|CallParentFunction DeltaSeconds))

(fn ConstructionScript
  (|CallParentFunction))